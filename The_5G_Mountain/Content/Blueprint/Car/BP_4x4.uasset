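; Drivable 4x4 vehicle with a winch that hooks a cable onto TreuilSapling actors.
; Enhanced Input feeds throttle, steering, brake and handbrake to the vehicle movement component, switches brake lights and toggles headlights.
; A per-tick sphere trace, aimed with the mouse-driven camera, remembers the last sapling hit.
; The winch input spawns a cable component attached to that sapling and flags it hooked; no pulling or release happens here.
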(event Input|EnhancedActionEvents|EnhancedInputActionIA_Steer
  (params (ActionValue :type Float%20%28double-precision%29) (ElapsedSeconds :type Float%20%28double-precision%29) (TriggeredSeconds :type Float%20%28double-precision%29) (InputAction :type Input%20Action%20Object%20Reference :default "/Game/Inputs/IA_Steer.IA_Steer"))
  (bind _vehiclemovementcomponent (Variables|Default|GetVehicleMovementComponent))
  (:Triggered
    (Class|ChaosVehicleMovementComponent|SetSteeringInput _vehiclemovementcomponent ActionValue))
  (:Completed
    (Class|ChaosVehicleMovementComponent|SetSteeringInput _vehiclemovementcomponent 0.0)))

(event Input|EnhancedActionEvents|EnhancedInputActionIA_Throttle
  (params (ActionValue :type Float%20%28double-precision%29) (ElapsedSeconds :type Float%20%28double-precision%29) (TriggeredSeconds :type Float%20%28double-precision%29) (InputAction :type Input%20Action%20Object%20Reference :default "/Game/Inputs/IA_Throttle.IA_Throttle"))
  (bind _vehiclemovementcomponent (Variables|Default|GetVehicleMovementComponent))
  (:Triggered
    (Class|ChaosVehicleMovementComponent|SetThrottleInput _vehiclemovementcomponent ActionValue))
  (:Completed
    (Class|ChaosVehicleMovementComponent|SetThrottleInput _vehiclemovementcomponent 0.0)))

(event Input|EnhancedActionEvents|EnhancedInputActionIA_Brake
  (params (ActionValue :type Float%20%28double-precision%29) (ElapsedSeconds :type Float%20%28double-precision%29) (TriggeredSeconds :type Float%20%28double-precision%29) (InputAction :type Input%20Action%20Object%20Reference :default "/Game/Inputs/IA_Brake.IA_Brake"))
  (bind _vehiclemovementcomponent (Variables|Default|GetVehicleMovementComponent))
  (:Triggered
    (Class|ChaosVehicleMovementComponent|SetBrakeInput _vehiclemovementcomponent ActionValue)
    (Variables|Default|SetIsBraking? true)
    (CallFunction|Brakelights :!label _label))
  (:Completed
    (Class|ChaosVehicleMovementComponent|SetBrakeInput _vehiclemovementcomponent 0.0)
    (Variables|Default|SetIsBraking? false)
    (goto _label)))

(event Input|EnhancedActionEvents|EnhancedInputActionMouse
  (params (ActionValue :type Vector%202D%20Structure) (ElapsedSeconds :type Float%20%28double-precision%29) (TriggeredSeconds :type Float%20%28double-precision%29) (InputAction :type Input%20Action%20Object%20Reference :default "/Game/Inputs/Mouse.Mouse"))
  (Pawn|Input|AddControllerYawInput (.x ActionValue))
  (Pawn|Input|AddControllerPitchInput (.y ActionValue))
  (Transformation|SetWorldRotation (Variables|Default|GetRaycast) (Class|SpringArmComponent|GetTargetRotation (Variables|Default|GetSpringArm)) false false))

(event Input|EnhancedActionEvents|EnhancedInputActionIA_Handbrake
  (params (ActionValue :type Boolean) (ElapsedSeconds :type Float%20%28double-precision%29) (TriggeredSeconds :type Float%20%28double-precision%29) (InputAction :type Input%20Action%20Object%20Reference :default "/Game/Inputs/IA_Handbrake.IA_Handbrake"))
  (bind _vehiclemovementcomponent (Variables|Default|GetVehicleMovementComponent))
  (:Started
    (Class|ChaosVehicleMovementComponent|SetHandbrakeInput _vehiclemovementcomponent true)
    (Variables|Default|SetIsBraking? true)
    (CallFunction|Brakelights :!label _label))
  (:Completed
    (Class|ChaosVehicleMovementComponent|SetHandbrakeInput _vehiclemovementcomponent false)
    (Variables|Default|SetIsBraking? false)
    (goto _label)))

(event Input|EnhancedActionEvents|EnhancedInputActionIA_Lights
  (params (ActionValue :type Boolean) (ElapsedSeconds :type Float%20%28double-precision%29) (TriggeredSeconds :type Float%20%28double-precision%29) (InputAction :type Input%20Action%20Object%20Reference :default "/Game/Inputs/IA_Lights.IA_Lights"))
  (bind _spotlight1 (Variables|Default|GetSpotLight1))
  (:Started
    (if (Variables|Default|GetLightOn?)
      (Variables|Default|SetLightOn? false)
      (Rendering|Components|Light|SetIntensity _spotlight1 0.0)
      (else
        (Variables|Default|SetLightOn? true)
        (Rendering|Components|Light|SetIntensity _spotlight1 1e+05)))))

(event Input|EnhancedActionEvents|EnhancedInputActionIA_Treuil
  (params (ActionValue :type Boolean) (ElapsedSeconds :type Float%20%28double-precision%29) (TriggeredSeconds :type Float%20%28double-precision%29) (InputAction :type Input%20Action%20Object%20Reference :default "/Game/Inputs/IA_Treuil.IA_Treuil"))
  (bind _cable (Variables|Default|GetCable))
  (bind _returnvalue (Transformation|GetWorldLocation _cable))
  (:Started
    (if (Utilities|IsValid (Variables|Default|GetLastSapling))
      (bind _returnvalue_2 (AddComponent|AddCableComponent false))
      (Transformation|SetWorldLocation _returnvalue_2 (Math|Vector|MakeVector (.x _returnvalue) (.y _returnvalue) (.z _returnvalue)) false false)
      (bind _output_get (Variables|Default|SetCableTreuil _returnvalue_2))
      (Variables|/Script/CableComponent.CableComponent|SetEndLocation _output_get "0, 0, 0")
      (Class|CableComponent|SetAttachEndtoComponent (Variables|Default|GetCableTreuil) (Variables|/Game/Blueprint/TreuilSapling.TreuilSapling_C|GetSphere (Variables|Default|GetLastSapling)) "Cube")
      (Variables|Default|SetCableAccroché true))))

(event EventTick
  (params (DeltaSeconds :type Float%20%28single-precision%29))
  (bind _raycast (Variables|Default|GetRaycast))
  (bind _returnvalue (Transformation|GetWorldLocation _raycast))
  (bind _outhit (Collision|SphereTraceByChannel _returnvalue (+ _returnvalue (* (Math|Vector|GetForwardVector _raycast) 5e+03)) 5e+01 "TraceTypeQuery1" false 0 "ForOneFrame"))
  (bind _astreuil_sapling (Utilities|Casting|CastToTreuilSapling (.hitactor _outhit)))
  (Variables|Default|SetLastSapling _astreuil_sapling))

(fn ConstructionScript)

(fn Brakelights
  (bind _rectlight (Variables|Default|GetRectLight))
  (if (Variables|Default|GetIsBraking?)
    (Rendering|Components|Light|SetIntensity _rectlight 1e+03)
    (else
      (Rendering|Components|Light|SetIntensity _rectlight 0.0))))