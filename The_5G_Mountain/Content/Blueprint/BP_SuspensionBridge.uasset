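; Suspension bridge actor that builds a physics-driven plank bridge along an editable spline.
; The construction script spawns plank meshes at fixed spacing along the spline and enables physics on each.
; On BeginPlay it links each neighbouring pair with a physics constraint at their midpoint, locking linear motion and limiting swing and twist.
; The first and last planks then stop simulating, anchoring both ends so the span can sag and sway.
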(event EventBeginPlay
  (bind _planks (Variables|Default|GetPlanks))
  (for _index (range 1 (- (Utilities|Array|Length (Variables|Default|GetPlanks)) 1))
    (bind _returnvalue (AddComponent|AddPhysicsConstraintComponent false))
    (Transformation|SetWorldLocation _returnvalue (Math|Vector|Lerp(Vector) (Transformation|GetWorldLocation (Utilities|Array|Get(acopy) _planks (- _index 1))) (Transformation|GetWorldLocation (Utilities|Array|Get(acopy) _planks _index)) 0.5) false false)
    (Class|PhysicsConstraintComponent|SetLinearXLimit _returnvalue "LCM_Locked" 0.0)
    (Class|PhysicsConstraintComponent|SetLinearYLimit _returnvalue "LCM_Locked" 0.0)
    (Class|PhysicsConstraintComponent|SetLinearZLimit _returnvalue "LCM_Locked" 0.0)
    (Class|PhysicsConstraintComponent|SetAngularSwing1Limit _returnvalue "ACM_Limited" 15.0)
    (Class|PhysicsConstraintComponent|SetAngularSwing2Limit _returnvalue "ACM_Limited" 5.0)
    (Class|PhysicsConstraintComponent|SetAngularTwistLimit _returnvalue "ACM_Limited" 5.0)
    (Class|PhysicsConstraintComponent|SetConstrainedComponents _returnvalue (Utilities|Array|Get(acopy) _planks (- _index 1)) "None" (Utilities|Array|Get(acopy) _planks _index) "None"))
  (Utilities|FlowControl|Sequence
    (:then_0
      (Physics|SetSimulatePhysics (Utilities|Array|Get(acopy) _planks) false))
    (:then_1
      (Physics|SetSimulatePhysics (Utilities|Array|Get(acopy) _planks (Utilities|Array|LastIndex _planks)) false))))

(fn ConstructionScript
  (for _index (range 0 (- (Math|Float|Floor (/ (Spline|GetSplineLength (Variables|Default|GetSplineComponent)) (Variables|Default|GetPlankSpacing))) 1))
    (bind _returnvalue (AddComponent|AddStaticMeshComponent false (Spline|GetTransformatDistanceAlongSpline (Variables|Default|GetSplineComponent) (* _index (Variables|Default|GetPlankSpacing)) "Local" false)))
    (Components|StaticMesh|SetStaticMesh _returnvalue (Variables|Default|GetPlankMesh))
    (Transformation|SetRelativeScale3D _returnvalue "0.800000,4.000000,0.150000")
    (Utilities|Array|Add (Variables|Default|GetPlanks) _returnvalue)
    (Physics|SetSimulatePhysics _returnvalue true)))