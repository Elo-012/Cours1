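; Main menu camera Blueprint that shows the menu UI and hands view and control over to the player's car.
; On BeginPlay it adds its UI widget to the viewport, sets itself as the widget's parent reference and shows the mouse cursor.
; Play runs once, blending the view to the CarPlayer stored in GI_Game, then possessing it after a matching delay.
; The throttle input only prints a debug string.
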(event Custom|Play
  (Utilities|FlowControl|DoOnce false
    (:Completed
      (bind _asgi_game (Utilities|Casting|CastToGI_Game (Game|GetGameInstance)))
      (Game|Player|SetViewTargetwithBlend (Game|GetPlayerController 0) (Variables|/Game/Blueprint/GI_Game.GI_Game_C|GetCarPlayer _asgi_game) 0.7 "VTBlend_Linear" 0.5 false)
      (Utilities|FlowControl|Delay 0.7)
      (Default|Possess (Variables|/Game/Blueprint/GI_Game.GI_Game_C|GetCarPlayer _asgi_game)))))

(event Input|EnhancedActionEvents|EnhancedInputActionIA_Throttle
  (params (ActionValue :type Float%20%28double-precision%29) (ElapsedSeconds :type Float%20%28double-precision%29) (TriggeredSeconds :type Float%20%28double-precision%29) (InputAction :type Input%20Action%20Object%20Reference :default "/Game/Inputs/IA_Throttle.IA_Throttle"))
  (Development|PrintString "Hello"))

(event EventBeginPlay
  (bind _ui (Variables|Default|GetUI))
  (UserInterface|Viewport|AddtoViewport _ui 0)
  (Variables|/Game/UI/MenuPrincipal.MenuPrincipal_C|Setparent _ui self)
  (Variables|/Script/Engine.PlayerController|SetbShowMouseCursor (Game|GetPlayerController 0) true))

(fn ConstructionScript)